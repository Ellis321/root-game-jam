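; BP_windSpawn is a spawner actor that periodically creates BP_wind actors at its Billboard component's transform.
; Tick feeds a random 10 to 20 second Delay, which acts as the repeat timer, then calls Shoot to spawn the wind.
; Debug strings print after each delay and shot.
; The Timer function is empty, and leftover timer and time-counter nodes are disconnected.
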(event `self.ReceiveBeginPlay`)

(event `self.ReceiveTick`
  (params (DeltaSeconds :type "Float (single-precision)"))
  (`KismetSystemLibrary.Delay` (`KismetMathLibrary.RandomFloatInRange` 10.0 20.0))
  (`KismetSystemLibrary.PrintString` "dleay")
  (`self.shoot`))

(fn `shoot`
  (`|SpawnActorFromClass` "/Game/Blue_print/BP_wind.BP_wind_C" (`SceneComponent.K2_GetComponentToWorld` (`self.Billboard`)) "Undefined" "OverrideRootScale" null null)
  (`KismetSystemLibrary.PrintString` "shot"))

(fn `timer`)

(fn `UserConstructionScript`)