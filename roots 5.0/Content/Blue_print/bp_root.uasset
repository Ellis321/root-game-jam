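; Player character for a platformer with side-to-side movement, jumping, wind knockback and a "rooting" ability, which also manages the start and win screens.
; Holding root traces a short ray from the camera and, on hitting a rootable platform, deactivates movement and swaps the cube's material until release.
; Wind-hit events apply strong sideways velocity impulses in either direction.
; Start and win events handle their widgets, and Escape quits the game.
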(event `win`
  ;[1 0 0.6385] stats
  (bind _returnvalue (`|CreateWidget` "/Game/wiget/winscreenn.winscreenn_C"))
  (bind _output_get (set `self.winscreen` _returnvalue))
  (`UserWidget.AddToViewport` _output_get 0))

(event `self.ReceiveBeginPlay`
  ;[1 0 0.6385] stats
  (bind _returnvalue (`|CreateWidget` "/Game/wiget/StartScreen.StartScreen_C"))
  (bind _output_get (set `self.start sreen` _returnvalue))
  (`UserWidget.AddToViewport` _output_get 0))

(event `start`
  ;[1 0 0.6385] stats
  (`GameplayStatics.SetViewportMouseCaptureMode` "NoCapture")
  (`Widget.RemoveFromParent` (`self.start sreen`)))

(event `windhit`
  ;[1 0.05042 0] HIT
  (`KismetSystemLibrary.PrintString` "wind it")
  (`CharacterMovementComponent.AddImpulse` (`self.CharacterMovement`) (* (`self.GetActorRightVector`) 3000.0) true))

(event `windhit left`
  ;[1 0.05042 0] HIT
  (`CharacterMovementComponent.AddImpulse` (`self.CharacterMovement`) (* (`self.GetActorRightVector`) -3000.0) true))

(event `InputAxis|left_rit`
  (params (AxisValue :type "Float (single-precision)"))
  ;[1 1 1] movement
  (`self.AddMovementInput` (`self.GetActorRightVector`) AxisValue))

(event `jumped`
  (params (jumped :type Boolean)))

(event `InputAction|rooting`
  (params (Key :type "Key Structure"))
  (bind _camera1 (`self.Camera1`))
  (bind _returnvalue (`SceneComponent.K2_GetComponentLocation` _camera1))
  ;[1 0.1438 0] rooting
  (:`Pressed`
    (bind _outhit (`KismetSystemLibrary.LineTraceSingle` :`Start` _returnvalue :`End` (+ (* (`KismetMathLibrary.GetForwardVector` (`SceneComponent.K2_GetComponentRotation` _camera1)) 25.0) _returnvalue) :`TraceChannel` "TraceTypeQuery2" :`DrawDebugType` "ForDuration"))
    (cast `/Game/Blue_print/BP_ROOTablePLAtform` (`.HitActor` (`GameplayStatics.BreakHitResult` _outhit)))
    (`ActorComponent.Deactivate` (`self.CharacterMovement`))
    (`PrimitiveComponent.SetMaterial` (`self.Cube`) 0 "/Game/material/stand_in_M.stand_in_M")
    (`KismetSystemLibrary.PrintString` "rooted"))
  (:`Released`
    (`PrimitiveComponent.SetMaterial` (`self.Cube`) 0 "/Game/material/MAT_M.MAT_M")
    (`ActorComponent.Activate` (`self.CharacterMovement`) false)))

(event `Key|Escape`
  (params (Key :type "Key Structure"))
  ;[1 1 1] movement
  (:`Pressed`
    (`KismetSystemLibrary.QuitGame` null "Quit")))

(event `InputAction|jump`
  (params (Key :type "Key Structure"))
  ;[1 1 1] movement
  (:`Pressed`
    (`self.Jump`)
    (`self.jumped` false)))

(fn `UserConstructionScript`)